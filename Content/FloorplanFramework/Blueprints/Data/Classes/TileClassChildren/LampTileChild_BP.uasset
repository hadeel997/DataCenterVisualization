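; LampTileChild_BP is a child tile class in the floorplan framework that acts as a lamp with a switchable point light.
; On BeginPlay, a timeline cosmetically fades the light intensity up from zero to full brightness.
; The Interactwith event uses a FlipFlop to snap the light off and on instantly, starting with off on the first use.
; Construction is left entirely to the parent class.
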(event EventBeginPlay
  ;[1 1 1] Fade Lamp In (Cosmetic Only)
  (bind _alpha (Timeline|LightBrightness PlayFromStart)
    (:Update
      (Rendering|Components|Light|SetIntensity (Variables|Default|GetPointLight) (Math|Float|Lerp 0.0 1e+03 _alpha)))
    (:Finished
      (Rendering|Components|Light|SetIntensity (Variables|Default|GetPointLight) 1e+03))))

(event EventInteractwith
  (bind _pointlight (Variables|Default|GetPointLight))
  (Utilities|FlowControl|FlipFlop
    (:A
      (Rendering|Components|Light|SetIntensity _pointlight 0.0))
    (:B
      (Rendering|Components|Light|SetIntensity _pointlight 1e+03))))

(fn ConstructionScript
  (|CallParentFunction))