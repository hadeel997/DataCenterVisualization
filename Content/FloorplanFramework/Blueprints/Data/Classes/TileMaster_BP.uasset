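; Base tile actor for the floorplan framework, representing a wall, floor or object.
; On update it takes mesh, materials and floor tag from the player controller, or restores them from load data; "NewFloor" tiles use a floor mesh and next-floor tag.
; Both paths then size collision from a data table, set responses by tile type and attach non-NewFloor tiles to the actor traced below.
; Events also handle painting, visibility and collision overrides.
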(event Custom|UpdateTile
  ;[1 0.6098 0.3229] Update Tile Events
  (|UpdateTileData)
  (|UpdateTileCollisionTransform)
  (|UpdateTileCollisionResponses)
  (|AttachActorToFloor))

(event Custom|OverrideCollision
  (params (Collision :type ECollisionEnabled%20Enum :default "NoCollision"))
  ;[1 0.6098 0.3229] Update Tile Events
  (|OverrideCollisionLogic Collision))

(event Custom|UpdateTileFromLoad
  (params (LoadData :type Save%20Data%20S%20Structure))
  ;[1 0.6098 0.3229] Update Tile Events
  (|UpdateDataOnLoad LoadData
    (:execute
      (|UpdateTileCollisionTransform)
      (|UpdateTileCollisionResponses)
      (|AttachActorToFloor))))

(event EventPaintTile
  (params (PaintMat :type Material%20Interface%20Object%20Reference))
  ;[1 0.6098 0.3229] Update Tile Events
  (|PaintTileLogic PaintMat))

(event EventSetVisibility
  (params (NewVisibility :type Boolean))
  ;[1 0.6098 0.3229] Update Tile Events
  (|UpdateVisibilityLogic NewVisibility))

(fn ConstructionScript)

(fn GetTileData
  (return (Variables|Default|GetTileData_S) (Variables|Default|GetFloor)))