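; Player pawn for the floorplan framework, providing the orbit camera and relaying editing hotkeys to the player controller.
; Each tick clamps pitch and spring-arm zoom, then lerps toward the average location of actors tagged with the current floor number.
; Camera mode 1 follows that point fully with movement disabled; mode 2 allows planar movement and follows only its height.
; It also creates the controls widget, toggles the content library and triggers layout save/load.
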(event Custom|CreatePawnBasedWidgets
  ;[0 0.5469 0.2384] Pawn Functions
  (bind _returnvalue (UserInterface|CreateWidget "/Game/FloorplanFramework/UserInterface/Widgets/Controls_W.Controls_W_C"))
  (bind _output_get (Variables|Default|SetControlsWidgetRef _returnvalue))
  (UserInterface|Viewport|AddtoViewport _output_get 0))

(event EventTick
  (params (DeltaSeconds :type Float%20%28single-precision%29))
  ;[0 0.5469 0.2384] Pawn Functions
  (Variables|Default|SetDeltaSeconds DeltaSeconds)
  (|ClampCameraValues)
  (|CameraMovement))

(event Input|ActionEvents|InputActionRemove
  (params (Key :type Key%20Structure))
  ;[0 0.5469 0.2384] Pawn Functions
  (:Pressed
    (Class|ControllerDataBPI|EditbyFunctionName(Message) (Game|GetPlayerController 0) "Delete")))

(event Input|ActionEvents|InputActionContentLibrary
  (params (Key :type Key%20Structure))
  ;[0 0.5469 0.2384] Pawn Functions
  (:Pressed
    (bind _contentlibrarywidgetref (Class|ControllerDataBPI|GetControllerData(Message) (Game|GetPlayerController 0)))
    (Default|ToggleContentLibrary _contentlibrarywidgetref)))

(event Input|ActionEvents|InputActionRotate
  (params (Key :type Key%20Structure))
  ;[0 0.5469 0.2384] Pawn Functions
  (:Pressed
    (Class|ControllerDataBPI|UpdateRelevantRotation(Message) (Game|GetPlayerController 0))))

(event Input|ActionEvents|InputActionChangeFloor
  (params (Key :type Key%20Structure))
  ;[0 0.5469 0.2384] Pawn Functions
  (:Pressed
    (Class|ControllerDataBPI|ChangeControllerFloor(Message) (Game|GetPlayerController 0) 1)))

(event Input|ActionEvents|InputActionCycleCameraMode
  (params (Key :type Key%20Structure))
  ;[0 0.5469 0.2384] Pawn Functions
  (:Pressed
    (|CycleCameraControlMode)))

(event Input|ActionEvents|InputActionSaveLayout
  (params (Key :type Key%20Structure))
  ;[0 0.5469 0.2384] Pawn Functions
  (:Pressed
    (|SaveLoad)))

(event Input|ActionEvents|InputActionLoadLayout
  (params (Key :type Key%20Structure))
  ;[0 0.5469 0.2384] Pawn Functions
  (:Pressed
    (|SaveLoad) ; enters at Load
  ))

(event Input|MouseEvents|RightMouseButton
  (params (Key :type Key%20Structure))
  ;[0 0.5469 0.2384] Pawn Functions
  (:Pressed
    (Variables|Default|SetIsRotateKeyHeld true))
  (:Released
    (Variables|Default|SetIsRotateKeyHeld false)))

(event Input|KeyboardEvents|1
  (params (Key :type Key%20Structure))
  ;[0 0.5469 0.2384] Pawn Functions
  (:Pressed
    (|UpdateControlMode)))

(event Input|KeyboardEvents|2
  (params (Key :type Key%20Structure))
  ;[0 0.5469 0.2384] Pawn Functions
  (:Pressed
    (|UpdateControlMode) ; enters at Index1
  ))

(event Input|KeyboardEvents|X
  (params (Key :type Key%20Structure))
  ;[0 0.5469 0.2384] Pawn Functions
  (:Pressed
    (Default|Toggle (Variables|Default|GetControlsWidgetRef))))

(event Input|KeyboardEvents|Escape
  (params (Key :type Key%20Structure))
  ;[0 0.5469 0.2384] Pawn Functions
  (:Pressed
    (Game|QuitGame 0 "Quit" false)))

(event Input|MouseEvents|RightMouseButton
  (params (Key :type Key%20Structure))
  ;[0 0.5469 0.2384] Pawn Functions
  (:Pressed
    (Class|ControllerDataBPI|InteractwithTileClass(Message) (Game|GetPlayerController 0))))

(fn ConstructionScript)

(event Input|AxisEvents|InputAxisRotHoz
  (params (AxisValue :type Float%20%28single-precision%29))
  ;[0.1302 0.1302 0.1302] Get the horizontal axis of the desired key/button and rotating the camera on that plane
  (if (Variables|Default|GetIsRotateKeyHeld)
    (Class|Actor|AddActorWorldRotation (Math|Rotator|MakeRotator 0.0 0.0 (* AxisValue (Variables|Default|GetRotSpeed))))))

(event Input|AxisEvents|InputAxisRotVert
  (params (AxisValue :type Float%20%28single-precision%29))
  ;[0.1302 0.1302 0.1302] Get the vertical axis of the desired key/button and rotating the camera on that plane
  (if (Variables|Default|GetIsRotateKeyHeld)
    (Transformation|AddActorLocalRotation (Math|Rotator|MakeRotator 0.0 (* AxisValue (Variables|Default|GetRotSpeed)) 0.0) false false)))

(event Input|AxisEvents|InputAxisMoveRight
  (params (AxisValue :type Float%20%28single-precision%29))
  ;[0.04688 0.04688 0.04688] Move Right/Left
  (Pawn|Input|AddMovementInput self (Math|Vector|GetRightVector (Math|Rotator|MakeRotator 0.0 0.0 (.yaw (Transformation|GetWorldRotation (Variables|Default|GetCamera))))) AxisValue true))

(event Input|AxisEvents|InputAxisMoveForward
  (params (AxisValue :type Float%20%28single-precision%29))
  ;[0.04688 0.04688 0.04688] Move Forward/Backwards
  (Pawn|Input|AddMovementInput self (Math|Vector|GetForwardVector (Math|Rotator|MakeRotator 0.0 0.0 (.yaw (Transformation|GetWorldRotation (Variables|Default|GetCamera))))) AxisValue true))

(event Input|ActionEvents|InputActionZoomIn
  (params (Key :type Key%20Structure))
  (:Pressed
    (|ZoomIn_2)))

(event Input|ActionEvents|InputActionZoomOut
  (params (Key :type Key%20Structure))
  (:Pressed
    (|ZoomOut_2)))

(event EventBeginPlay
  (CallFunction|CreatePawnBasedWidgets)
  (CallFunction|UpdateCameraMode 1))

(event Custom|UpdateCameraMode
  (params (ForcedNewMode :type Integer))
  (bind _output_get (Variables|Default|SetCameraMode ForcedNewMode))
  (switch int _output_get
    (:1
      (Components|Activation|Deactivate (Variables|Default|GetPawnMovement)))
    (:2
      (Components|Activation|Activate (Variables|Default|GetPawnMovement) false))))