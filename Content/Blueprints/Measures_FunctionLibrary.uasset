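; Measures_FunctionLibrary is a function library that classifies integer Weight and Temp readings into enum categories.
; JudgeWeight and JudgeTemp each chain integer range checks to pick one of three bands, with a fourth value as the fallback.
; The lower two bands match in both functions, but Weight's top band starts higher, so values between its middle and top bands get the fallback.
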(fn JudgeWeight
  (params (Weight :type Integer))
  (if (Math|Integer|InRange(Integer) Weight 0 30)
    (return "NewEnumerator2")
    (elif (Math|Integer|InRange(Integer) Weight 30 70)
      (return "NewEnumerator1")
      (elif (Math|Integer|InRange(Integer) Weight 100 200)
        (return "NewEnumerator0")
        (else
          (return "NewEnumerator3"))))))

(fn JudgeTemp
  (params (Temp :type Integer))
  (if (Math|Integer|InRange(Integer) Temp 0 30)
    (return "NewEnumerator2")
    (elif (Math|Integer|InRange(Integer) Temp 30 70)
      (return "NewEnumerator1")
      (elif (Math|Integer|InRange(Integer) Temp 70 120)
        (return "NewEnumerator0")
        (else
          (return "NewEnumerator3"))))))