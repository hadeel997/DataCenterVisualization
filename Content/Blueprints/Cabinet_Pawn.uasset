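; Cabinet_Pawn is a camera pawn with look and zoom controls driven by Enhanced Input.
; On BeginPlay it adds the IMC_RTS mapping context through Main_Playercontroller's input subsystem.
; Look input drives controller yaw and inverted pitch, while zoom changes the spring arm length in scaled steps, ignoring any step outside a fixed range.
; The StartLooking input event is an empty stub.
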(event Input|EnhancedActionEvents|EnhancedInputActionIA_Look
  (params (ActionValue :type Vector%202D%20Structure) (ElapsedSeconds :type Float%20%28double-precision%29) (TriggeredSeconds :type Float%20%28double-precision%29) (InputAction :type Input%20Action%20Object%20Reference :default "/Game/Blueprints/Input/IA_Look.IA_Look"))
  (Pawn|Input|AddControllerYawInput (.x ActionValue))
  (Pawn|Input|AddControllerPitchInput (* (.y ActionValue) -1.0)))

(event Input|EnhancedActionEvents|EnhancedInputActionIA_StartLooking
  (params (ActionValue :type Boolean) (ElapsedSeconds :type Float%20%28double-precision%29) (TriggeredSeconds :type Float%20%28double-precision%29) (InputAction :type Input%20Action%20Object%20Reference :default "/Game/Blueprints/Input/IA_StartLooking.IA_StartLooking")))

(event Input|EnhancedActionEvents|EnhancedInputActionIA_Zoom
  (params (ActionValue :type Float%20%28double-precision%29) (ElapsedSeconds :type Float%20%28double-precision%29) (TriggeredSeconds :type Float%20%28double-precision%29) (InputAction :type Input%20Action%20Object%20Reference :default "/Game/IA_Zoom.IA_Zoom"))
  (bind _springarm (Variables|Default|GetSpringArm))
  (if (Math|Float|InRange(Float) (+ (* ActionValue 2e+01) (Variables|/Script/Engine.SpringArmComponent|GetTargetArmLength _springarm)) 2.5e+02 1e+03)
    (Variables|/Script/Engine.SpringArmComponent|SetTargetArmLength _springarm (+ (* ActionValue 2e+01) (Variables|/Script/Engine.SpringArmComponent|GetTargetArmLength _springarm)))))

(event EventBeginPlay
  (Utilities|FlowControl|Sequence
    (:then_0
      (bind _asmain_playercontroller (Utilities|Casting|CastToMain_Playercontroller (Game|GetPlayerController 0)))
      (Utilities|IsValid (PlayerController|LocalPlayerSubsystems|GetEnhancedInputLocalPlayerSubsystem _asmain_playercontroller)
        (:Is%20Valid
          (Input|AddMappingContext (PlayerController|LocalPlayerSubsystems|GetEnhancedInputLocalPlayerSubsystem _asmain_playercontroller) "/Game/Blueprints/Input/IMC_RTS.IMC_RTS" 0 "(bIgnoreAllPressedKeysUntilRelease=True,bForceImmediately=False,bNotifyUserSettings=False)"))))))

(fn ConstructionScript)