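; Heat map actor that paints splats into a render target at the locations of Cabinet_BP actors, with random strength.
; Key 1 generates the map and key 2 clears it to black.
; Each world location becomes plane-relative, is divided by Resolution, made absolute, then fed to a dynamic M_HeatSplat material drawn into the target.
; A line-trace path for painting at the player's position is disconnected and never runs.
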(event Custom|DrawToRenderTarget
  (params (Location :type Vector) (Strength :type Float%20%28double-precision%29) (Size :type Float%20%28double-precision%29))
  (bind _plane (Variables|Default|GetPlane))
  (bind _returnvalue (Transformation|GetWorldTransform _plane))
  (Rendering|Material|SetScalarParameterValue (Variables|Default|GetMI_HeatSplat) "Strength" Strength :!class /Script/Engine.MaterialInstanceDynamic)
  (Rendering|Material|SetScalarParameterValue (Variables|Default|GetMI_HeatSplat) "Size" Size :!class /Script/Engine.MaterialInstanceDynamic)
  (Rendering|Material|SetVectorParameterValue (Variables|Default|GetMI_HeatSplat) "Position" (Math|Conversions|ToLinearColor(Vector) (Math|Vector|VectorGetAbs (/ (Math|Transform|TransformLocation (Math|Transform|InvertTransform (Math|Transform|MakeTransform (.location _returnvalue) (.rotation _returnvalue) "1.000000,1.000000,1.000000")) Location) (Variables|Default|GetResolution)))) :!class /Script/Engine.MaterialInstanceDynamic)
  (Rendering|DrawMaterialtoRenderTarget (Variables|Default|GetRenderTarget) (Variables|Default|GetMI_HeatSplat)))

(event Custom|GenerateHeatMap
  (bind _outactors (Actor|GetAllActorsOfClass "/Game/Blueprints/Cabinet_BP.Cabinet_BP_C"))
  (for _array_element _outactors
    (Development|PrintString "Hello")
    (CallFunction|DrawtoRenderTarget (Transformation|GetActorLocation _array_element) (Math|Random|RandomFloatinRange 5.0 1e+01) 0.5)))

(event EventTick
  (params (DeltaSeconds :type Float%20%28single-precision%29))
  (Utilities|IsValid (Variables|Default|GetplayerRef)))

(event EventBeginPlay
  (Input|EnableInput (Game|GetPlayerController 0)))

(event Input|KeyboardEvents|2
  (params (Key :type Key%20Structure :default "None"))
  (:Pressed
    (Rendering|ClearRenderTarget2D (Variables|Default|GetRenderTarget))))

(event Input|KeyboardEvents|1
  (params (Key :type Key%20Structure :default "None"))
  (:Pressed
    (CallFunction|GenerateHeatMap)))

(fn ConstructionScript
  (bind _returnvalue (Rendering|Material|CreateDynamicMaterialInstance "/Game/Assets/Materials/HeatMap/M_HeatSplat.M_HeatSplat" "None" "None" :!class /Script/Engine.KismetMaterialLibrary))
  (Variables|Default|SetMI_HeatSplat _returnvalue))