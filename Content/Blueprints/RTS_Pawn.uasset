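; RTS_Pawn is a player pawn for an RTS-style view that turns the controller's yaw and pitch from look input.
; On BeginPlay it adds the RTS input mapping context and binds to the main UI's report-change event through Main_Playercontroller.
; When the report changes, it spawns a fresh RTS_Pawn at its location, has the controller possess it, then destroys itself.
; The start-looking input event is empty.
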(event Custom|CustomEvent
  (params (Report%20Type :type E_ReportType%20Enum :default "NewEnumerator0"))
  (bind _returnvalue (Game|SpawnActorfromClass "RTS_Pawn_C" (Math|Transform|MakeTransform (Transformation|GetActorLocation) "0, 0, 0" "1.000000,1.000000,1.000000") "Undefined" "MultiplyWithRoot" 0 0))
  (Pawn|Possess (stale EventBeginPlay _asmain_playercontroller) _returnvalue)
  (Actor|DestroyActor))

(event Input|EnhancedActionEvents|EnhancedInputActionIA_Look
  (params (ActionValue :type Vector%202D%20Structure) (ElapsedSeconds :type Float%20%28double-precision%29) (TriggeredSeconds :type Float%20%28double-precision%29) (InputAction :type Input%20Action%20Object%20Reference :default "/Game/Blueprints/Input/IA_Look.IA_Look"))
  (Pawn|Input|AddControllerYawInput (.x ActionValue))
  (Pawn|Input|AddControllerPitchInput (* (.y ActionValue) -1.0)))

(event Input|EnhancedActionEvents|EnhancedInputActionIA_StartLooking
  (params (ActionValue :type Boolean) (ElapsedSeconds :type Float%20%28double-precision%29) (TriggeredSeconds :type Float%20%28double-precision%29) (InputAction :type Input%20Action%20Object%20Reference :default "/Game/Blueprints/Input/IA_StartLooking.IA_StartLooking")))

(event EventBeginPlay
  (Utilities|FlowControl|Sequence
    (:then_0
      (bind _asmain_playercontroller (Utilities|Casting|CastToMain_Playercontroller (Game|GetPlayerController 0)))
      (Utilities|IsValid (PlayerController|LocalPlayerSubsystems|GetEnhancedInputLocalPlayerSubsystem _asmain_playercontroller)
        (:Is%20Valid
          (Input|AddMappingContext (PlayerController|LocalPlayerSubsystems|GetEnhancedInputLocalPlayerSubsystem _asmain_playercontroller) "/Game/Blueprints/Input/IMC_RTS.IMC_RTS" 0 "(bIgnoreAllPressedKeysUntilRelease=True,bForceImmediately=False,bNotifyUserSettings=False)")
          (EventDispatchers|BindEventtoChangeReport (Variables|/Game/Blueprints/Main_Playercontroller.Main_Playercontroller_C|GetMain%20UI%20Ref _asmain_playercontroller) (delegate Custom|CustomEvent)))))))

(fn ConstructionScript)