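; Manager actor that spawns and controls a set of cabinets laid out along a spline.
; On BeginPlay it spawns one Cabinet_BP per data table row at the matching spline point, then passes the list to its JSON component.
; A looping half-second timer polls that component's JSON data to switch each cabinet's warning light by ID.
; Animatecabinates plays the dive animation state on every cabinet except the excepted ID.
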(event Custom|Animate%20cabinates
  (params (Dive? :type Boolean) (ID%20Exeption :type String))
  (for _array_element (Variables|Default|GetCabinets)
    (if (not (Utilities|Enum|Equal(Enum) ID%20Exeption (.id (Variables|/Game/Blueprints/Cabinet_BP.Cabinet_BP_C|GetCabinetData _array_element))))
      (Default|AnimateCabinate _array_element Dive?))))

(event Custom|CustomEvent
  (bind _data (Default|ReadfromJson (Variables|Default|GetJson_Comp)))
  (for _array_element (.cabenitesdata _data)
    (Default|TurnWarningLight (Utilities|Array|Get(acopy) (Variables|Default|GetCabinets) (.ID (Utilities|Struct|BreakF_JsonData _array_element))) (.WarningLightsOn (Utilities|Struct|BreakF_JsonData _array_element)))))

(event EventBeginPlay
  (bind _cabinetdatatable (Variables|Default|GetCabinetDataTable))
  (bind _outrownames (DataTable|GetDataTableRowNames _cabinetdatatable))
  (for (_array_element _array_index) _outrownames
    (bind _returnvalue (Utilities|GetDataTableRow _cabinetdatatable _array_element)
      (:then
        (bind _returnvalue_2 (Game|SpawnActorfromClass "/Game/Blueprints/Cabinet_BP.Cabinet_BP_C" (Math|Transform|MakeTransform (Spline|GetLocationatSplinePoint (Variables|Default|GetSpline) _array_index "World") "0, 0, 0" "1.000000,1.000000,1.000000") "Undefined" "MultiplyWithRoot" 0 _returnvalue 0))
        (Utilities|Array|Add (Variables|Default|GetCabinets) _returnvalue_2))))
  (Default|Init (Variables|Default|GetJson_Comp) (Variables|Default|GetCabinets))
  (Utilities|Time|SetTimerbyEvent (delegate Custom|CustomEvent) 0.5 true))

(fn ConstructionScript)