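; Json component that saves and loads per-cabinet data (an ID and a warning-light flag) in a JSON file at JsonPath.
; Init adds an entry per array index of the passed cabinets with lights off, then converts the struct to JSON and writes the file.
; ReadFromJson clears the data, rebuilds it field by field from the file and returns it.
; The writetojsonfile event is an empty stub.
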(event Custom|write%20to%20json%20file
  (params (Struct :type F%20Json%20Data%20Structure) (Path :type String)))

(event Custom|Init
  (params (ArrayOfCabs :type Array%20of%20Cabinet%20BP%20Object%20References))
  (bind _output_get (Variables|Default|SetArrayOfCabs ArrayOfCabs))
  (for (_ _array_index) _output_get
    (bind _output_get_2 (Variables|Default|SetFile%20Data (Utilities|Struct|MakeF_JsonData _array_index false)))
    (Utilities|Array|Add (.cabenitesdata (Variables|Default|Getdata)) _output_get_2))
  (bind _outjsonstring (|StructtoJsonString (Variables|Default|Getdata)))
  (bind _outjsonobject (Class|JsonBlueprintFunctionLibrary|FromString _outjsonstring))
  (Class|JsonBlueprintFunctionLibrary|ToFile _outjsonobject (Utilities|Struct|MakeFilePath (Class|BlueprintPathsLibrary|ConvertRelativePathtoFull (Variables|Default|GetJson%20Path)))))

(event EventBeginPlay)

(fn ReadfromJson
  (Utilities|Array|Clear (.cabenitesdata (Variables|Default|Getdata)))
  (bind _outjsonobject (Class|JsonBlueprintFunctionLibrary|FromFile (Utilities|Struct|MakeFilePath (Class|BlueprintPathsLibrary|ConvertRelativePathtoFull (Variables|Default|GetJson%20Path)))))
  (bind _outvalue (|GetJsonField _outjsonobject "CabenitesData"))
  (for _array_element _outvalue
    (bind _outvalue_2 (|GetJsonField _array_element "iD"))
    (bind _outvalue_3 (|GetJsonField _array_element "warningLightsOn"))
    (Utilities|Array|Add (.cabenitesdata (Variables|Default|Getdata)) (Utilities|Struct|MakeF_JsonData (Class|KismetSystemLibrary|MakeLiteralInteger _outvalue_2) _outvalue_3)))
  (return (Variables|Default|Getdata)))